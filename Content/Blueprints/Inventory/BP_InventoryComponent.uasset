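; Inventory component holding hotbar and backpack slot maps, with item search (hotbar first) and empty-slot lookup.
; Slots count as empty when the item's icon is invalid.
; MoveItemToNewSlot stacks matching IDs, swaps different items or moves into empty slots, returning resulting slot data without writing the maps.
; SelectAndFireDelegate maps an enum to added/removed dispatchers for hotbar, backpack or other inventory, notifying listeners such as MainOverlay.
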(event `self.ReceiveBeginPlay`
  (set `self.OwnerOfInventory` (`self.GetOwner`)))

(fn `CheckHotbarSpace`
  (returns (DoesHotbarHaveSpace :type Boolean))
  (locals (`DoesHotbarHaveSpace?` :type Boolean))
  (bind _values (`BlueprintMapLibrary.Map_Values` (`self.HotbarInventory`)))
  (for _array_element _values
    (if (`KismetSystemLibrary.IsValid` (`.Icon_18_5A4333B14DC05DD507265FB7F709CEBC` (break `/Game/Blueprints/Inventory/Data/Struct_Item` (`.Item_2_9C6C3E8D4CDA4446392BBD8E68208A25` (break `/Game/Blueprints/Inventory/Data/Struct_InventorySlotData` _array_element)))))
      (set `local.DoesHotbarHaveSpace?` false)
      (else
        (set `local.DoesHotbarHaveSpace?` true)
        (break))))
  (return (`local.DoesHotbarHaveSpace?`)))

(fn `FindEmptyBackpackSlot`
  (returns (EmptyBackpackSlot :type Integer))
  (locals (EmptySlot :type Integer))
  (bind _values (`BlueprintMapLibrary.Map_Values` (`self.BackpackInventory`)))
  (for (_array_element _array_index) _values
    (if (not (`KismetSystemLibrary.IsValid` (`.Icon_18_5A4333B14DC05DD507265FB7F709CEBC` (break `/Game/Blueprints/Inventory/Data/Struct_Item` (`.Item_2_9C6C3E8D4CDA4446392BBD8E68208A25` (break `/Game/Blueprints/Inventory/Data/Struct_InventorySlotData` _array_element))))))
      (set `local.EmptySlot` _array_index)
      (break)))
  (return (`local.EmptySlot`)))

(fn `FindEmptyHotbarSlot`
  (returns (EmptyHotbarSlot :type Integer))
  (locals (EmptySlot :type Integer :default 0))
  (bind _values (`BlueprintMapLibrary.Map_Values` (`self.HotbarInventory`)))
  (for (_array_element _array_index) _values
    (if (not (`KismetSystemLibrary.IsValid` (`.Icon_18_5A4333B14DC05DD507265FB7F709CEBC` (break `/Game/Blueprints/Inventory/Data/Struct_Item` (`.Item_2_9C6C3E8D4CDA4446392BBD8E68208A25` (break `/Game/Blueprints/Inventory/Data/Struct_InventorySlotData` _array_element))))))
      (set `local.EmptySlot` _array_index)
      (break)))
  (return (`local.EmptySlot`)))

(fn `FindItem`
  (params (Item :type "/Game/Blueprints/Inventory/Data/Struct_Item Structure"))
  (returns (WasItemFound :type Boolean) (FromHotbar :type Boolean) (FoundItemSlot :type "/Game/Blueprints/Inventory/Data/Struct_InventorySlotData Structure") (FoundIndex :type Integer))
  (locals (FoundItem_Local :type "/Game/Blueprints/Inventory/Data/Struct_InventorySlotData Structure") (FoundIndex_Local :type Integer) (`WasItemInHotbar?_Local` :type Boolean) (FoundQuantity_Local :type Integer) (`WasItemFound?_Local` :type Boolean))
  (bind _values (`BlueprintMapLibrary.Map_Values` (`self.HotbarInventory`)))
  (bind (_founditem _wasitemfound_ _foundindex) (`self.FindItemInSpecificInventory` _values (`local.Item`)))
  (set `local.FoundItem_Local` _founditem)
  (set `local.WasItemFound?_Local` _wasitemfound_)
  (set `local.FoundIndex_Local` _foundindex)
  (if _wasitemfound_
    (return (`local.WasItemFound?_Local`) true (`local.FoundItem_Local`) (`local.FoundIndex_Local`))
    (else
      (bind _values_2 (`BlueprintMapLibrary.Map_Values` (`self.BackpackInventory`)))
      (bind (_founditem_2 _wasitemfound__2 _foundindex_2) (`self.FindItemInSpecificInventory` _values_2 (`local.Item`)))
      (set `local.FoundItem_Local` _founditem_2)
      (set `local.FoundIndex_Local` _foundindex_2)
      (return _wasitemfound__2 false (`local.FoundItem_Local`) (`local.FoundIndex_Local`)))))

(fn `FindItemInSpecificInventory`
  (params (InventoryValues :type "Array of /Game/Blueprints/Inventory/Data/Struct_InventorySlotData Structure") (Item :type "/Game/Blueprints/Inventory/Data/Struct_Item Structure"))
  (returns (FoundItem :type "/Game/Blueprints/Inventory/Data/Struct_InventorySlotData Structure") (`WasItemFound?` :type Boolean) (FoundIndex :type Integer))
  (locals (FoundQuantity_Local :type Integer) (`WasItemFound?_Local` :type Boolean) (`WasItemInHotbar?_Local` :type Boolean) (FoundIndex_Local :type Integer) (FoundItem_Local :type "/Game/Blueprints/Inventory/Data/Struct_InventorySlotData Structure"))
  (for (_array_element _array_index) InventoryValues
    (bind (_item _quantity) (break `/Game/Blueprints/Inventory/Data/Struct_InventorySlotData` _array_element))
    (if (== (`.ID_37_2860070F4E14361ABD215881AD40851C` (break `/Game/Blueprints/Inventory/Data/Struct_Item` _item)) (`.ID_37_2860070F4E14361ABD215881AD40851C` (break `/Game/Blueprints/Inventory/Data/Struct_Item` (`local.Item`))))
      (set `local.FoundItem_Local` _array_element)
      (set `local.FoundIndex_Local` _array_index)
      (set `local.WasItemFound?_Local` true)
      (set `local.FoundQuantity_Local` _quantity)
      (break)
      (else
        (set `local.WasItemFound?_Local` false))))
  (return (`local.FoundItem_Local`) (`local.WasItemFound?_Local`) (`local.FoundIndex_Local`)))

(fn `MoveItemToNewSlot`
  (params (FromSlot :type Integer) (ToSlot :type Integer) (ToInventory :type "Map of Integer to /Game/Blueprints/Inventory/Data/Struct_InventorySlotData Structure") (FromInventory :type "Map of Integer to /Game/Blueprints/Inventory/Data/Struct_InventorySlotData Structure") (FromInventoryComponent :type "/Game/Blueprints/Inventory/BP_InventoryComponent Object Reference") (ToInventoryComponent :type "/Game/Blueprints/Inventory/BP_InventoryComponent Object Reference") (TO_Delegate :type "/Game/Blueprints/Inventory/Data/Enum_IconDelegates Enum" :default "NewEnumerator0") (FROM_Delegate :type "/Game/Blueprints/Inventory/Data/Enum_IconDelegates Enum" :default "NewEnumerator0"))
  (returns (ItemFrom_FROM_Slot :type "/Game/Blueprints/Inventory/Data/Struct_InventorySlotData Structure") (ItemFrom_TO_Slot :type "/Game/Blueprints/Inventory/Data/Struct_InventorySlotData Structure"))
  (locals (ItemInToSlot :type Boolean) (`SlotsInSameInventory?` :type Boolean) (EnumSelection :type "/Game/Blueprints/Inventory/Data/Enum_IconDelegates Enum" :default "NewEnumerator0") (SavedItemInToSlot :type "/Game/Blueprints/Inventory/Data/Struct_InventorySlotData Structure") (SavedItemInFromSlot :type "/Game/Blueprints/Inventory/Data/Struct_InventorySlotData Structure") (ToSlotItemID :type Integer) (FromSlotItemID :type Integer))
  (bind _savediteminfromslot (`local.SavedItemInFromSlot`))
  (bind _value (`BlueprintMapLibrary.Map_Find` (`local.ToInventory`) (`local.ToSlot`)))
  (bind _value_2 (`BlueprintMapLibrary.Map_Find` (`local.FromInventory`) (`local.FromSlot`)))
  (bind (_id _name _icon) (break `/Game/Blueprints/Inventory/Data/Struct_Item` (`.Item_2_9C6C3E8D4CDA4446392BBD8E68208A25` (break `/Game/Blueprints/Inventory/Data/Struct_InventorySlotData` _value))))
  ;[0 0 0] If the player picks up the item and drops it in the same slot, do nothing
  (if (and (== (`local.ToSlot`) (`local.FromSlot`)) (== (`local.FromInventoryComponent`) (`local.ToInventoryComponent`)))
    ;[0 0 0] Return exactly what was input
    (return (`BlueprintMapLibrary.Map_Find` (`local.FromInventory`) (`local.FromSlot`)) (`BlueprintMapLibrary.Map_Find` (`local.ToInventory`) (`local.ToSlot`)))
    (else
      (`|ExecutionSequence`
        (:`then_0`
          ;[0 0 0] Set variables based on items in to and from slots
          (set `local.ToSlotItemID` _id)
          (set `local.SavedItemInToSlot` _value)
          (set `local.ItemInToSlot` (`KismetSystemLibrary.IsValid` _icon)))
        (:`then_1`
          (set `local.FromSlotItemID` (`.ID_37_2860070F4E14361ABD215881AD40851C` (break `/Game/Blueprints/Inventory/Data/Struct_Item` (`.Item_2_9C6C3E8D4CDA4446392BBD8E68208A25` (break `/Game/Blueprints/Inventory/Data/Struct_InventorySlotData` _value_2)))))
          (set `local.SavedItemInFromSlot` _value_2)
          ;[0 0 0] If "to" slot has an item:
          (if (`local.ItemInToSlot`)
            ;[0 0 0] Do the items have the same ID? Should we stack?
            (if (== (`local.ToSlotItemID`) (`local.FromSlotItemID`))
              ;[0 0 0] Stack item
              (`|ExecutionSequence`
                (:`then_0`
                  ;;[0.05 0.05 0.05] Add the "from" and "to" slot's quantities together, and add them back into the "to" slot (stack the item). Call the generic dispatcher to notify MainOverlay of change
                  (bind _structout (setmembers `/Game/Blueprints/Inventory/Data/Struct_InventorySlotData` :`StructRef` _savediteminfromslot :`Quantity` (+ (`.Quantity_5_8D1E399245DFF28C8697A8BA5EC5307F` (break `/Game/Blueprints/Inventory/Data/Struct_InventorySlotData` _savediteminfromslot)) (`.Quantity_5_8D1E399245DFF28C8697A8BA5EC5307F` (break `/Game/Blueprints/Inventory/Data/Struct_InventorySlotData` (`local.SavedItemInToSlot`))))))
                  (`self.SelectAndFireDelegate` (`local.TO_Delegate`) (struct) (`local.ToSlot`) (`local.ToInventoryComponent`)))
                (:`then_1`
                  ;;[0.05 0.05 0.05] Replace the item in the "from" slot with an empty item. Call the dispatcher to change icons.
                  (`self.SelectAndFireDelegate` (`local.FROM_Delegate`) (make `/Game/Blueprints/Inventory/Data/Struct_InventorySlotData` (`self.EmptyItem`)) (`local.FromSlot`) (`local.FromInventoryComponent`))
                  (return _structout (make `/Game/Blueprints/Inventory/Data/Struct_InventorySlotData` (`self.EmptyItem`)))))
              (else
                ;[0 0 0] Swap Items
                (`|ExecutionSequence`
                  (:`then_0`
                    ;;[0.05 0.05 0.05] Add the item from the "from" slot to the "to" slot
                    (`self.SelectAndFireDelegate` (`local.TO_Delegate`) (`local.SavedItemInFromSlot`) (`local.ToSlot`) (`local.ToInventoryComponent`)))
                  (:`then_1`
                    ;;[0.05 0.05 0.05] Fires "Added to" delegates instead of "Removed from" so the icons aren't cleared
                    (switch `/Game/Blueprints/Inventory/Data/Enum_IconDelegates` (`local.FROM_Delegate`)
                      (:`NewEnumerator3`
                        (set `local.EnumSelection` "NewEnumerator0"))
                      (:`NewEnumerator4`
                        (set `local.EnumSelection` "NewEnumerator1"))
                      (:`NewEnumerator5`
                        (set `local.EnumSelection` "NewEnumerator2")))
                    (`self.SelectAndFireDelegate` (`local.EnumSelection`) (`local.SavedItemInToSlot`) (`local.FromSlot`) (`local.FromInventoryComponent`))
                    (return (`local.SavedItemInFromSlot`) (`local.SavedItemInToSlot`))))))
            (else
              (`|ExecutionSequence`
                (:`then_0`
                  ;[0 0 0] Add the item from the "from" slot to the "to" slot
                  (`self.SelectAndFireDelegate` (`local.TO_Delegate`) (`local.SavedItemInFromSlot`) (`local.ToSlot`) (`local.ToInventoryComponent`)))
                (:`then_1`
                  ;[0 0 0] Replace the item in the "from" slot with an empty item
                  (`self.SelectAndFireDelegate` (`local.FROM_Delegate`) (struct) (`local.FromSlot`) (`local.ToInventoryComponent`))
                  (return (`local.SavedItemInFromSlot`) (make `/Game/Blueprints/Inventory/Data/Struct_InventorySlotData` (`self.EmptyItem`))))))))))))

(fn `RemoveAllItemsFromBackpackInventory`
  (params (DelegateToFire :type "/Game/Blueprints/Inventory/Data/Enum_IconDelegates Enum" :default "NewEnumerator0") (OtherInventory :type "/Game/Blueprints/Inventory/BP_InventoryComponent Object Reference"))
  (bind _values (`BlueprintMapLibrary.Map_Values` (`self.BackpackInventory`)))
  (for (_array_element _array_index) _values
    (if (`KismetSystemLibrary.IsValid` (`.Icon_18_5A4333B14DC05DD507265FB7F709CEBC` (break `/Game/Blueprints/Inventory/Data/Struct_Item` (`.Item_2_9C6C3E8D4CDA4446392BBD8E68208A25` (break `/Game/Blueprints/Inventory/Data/Struct_InventorySlotData` _array_element)))))
      (`BlueprintMapLibrary.Map_Add` (`self.HotbarInventory`) _array_index (make `/Game/Blueprints/Inventory/Data/Struct_InventorySlotData` (`self.EmptyItem`)))
      (`self.SelectAndFireDelegate` (`local.DelegateToFire`) (struct) _array_index (`local.OtherInventory`)))))

(fn `SelectAndFireDelegate`
  (params (Selection :type "/Game/Blueprints/Inventory/Data/Enum_IconDelegates Enum" :default "NewEnumerator0") (ItemSlot :type "/Game/Blueprints/Inventory/Data/Struct_InventorySlotData Structure") (SlotIndex :type Integer) (OtherInventory :type "/Game/Blueprints/Inventory/BP_InventoryComponent Object Reference"))
  (bind (_itemslot_item _itemslot_quantity) (break `/Game/Blueprints/Inventory/Data/Struct_InventorySlotData` (`local.ItemSlot`)))
  (bind (_itemslot_item_2 _itemslot_quantity_2) (break `/Game/Blueprints/Inventory/Data/Struct_InventorySlotData` (`local.ItemSlot`)))
  (switch `/Game/Blueprints/Inventory/Data/Enum_IconDelegates` Selection
    (:`NewEnumerator0`
      (`self.ItemAddedToBackpack` (`local.ItemSlot`) (`local.SlotIndex`)))
    (:`NewEnumerator1`
      (`self.ItemAddedToHotbar` _itemslot_item_2 (`local.SlotIndex`) _itemslot_quantity_2))
    (:`NewEnumerator2`
      (`self.ItemAddedToOtherInventory` _itemslot_item _itemslot_quantity (`local.SlotIndex`) (`local.OtherInventory`)))
    (:`NewEnumerator3`
      (`self.ItemRemovedFromBackpack` (struct) (`local.SlotIndex`)))
    (:`NewEnumerator4`
      (`self.ItemRemovedFromHotbar` (struct) (`local.SlotIndex`)))
    (:`NewEnumerator5`
      (`self.ItemRemovedFromOtherInventory` (`local.SlotIndex`)))))