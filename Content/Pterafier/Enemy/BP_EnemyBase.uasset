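; Base melee enemy character that attacks the player, reacts to hits and exposes patrol route and speed settings to AI.
; Attack plays a montage whose notify moves an overlap detector forward and damages the PlayerState rather than the player pawn.
; Incoming damage reports to AI perception, then triggers hit effects and a movement-pausing montage.
; Death sets a Blackboard flag, ragdolls the mesh with an impulse along the player's facing, then destroys the actor.
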(event `self.ReceiveBeginPlay`
  (add `self.OnTakeAnyDamage` (delegate `OnTakeAnyDamage_Event`))
  (set `self.Health` (`self.MaxHealth`))
  (bind _asbp_third_person_character (cast `/Game/ThirdPersonTemplate/ThirdPerson/Blueprints/BP_ThirdPersonCharacter` (`GameplayStatics.GetPlayerCharacter` 0)))
  (set `self.PlayerRef` _asbp_third_person_character)
  (bind _asbp_player_state (cast `/Game/ThirdPersonTemplate/ThirdPerson/Blueprints/BP_PlayerState` (`GameplayStatics.GetPlayerState` 0)))
  (set `self.PlayerStateRef` _asbp_player_state)
  (set `CharacterMovementComponent.MaxWalkSpeed` (`KismetMathLibrary.RandomFloatInRange` 150.0 325.0) (`self.CharacterMovement`)))

(event `OnTakeAnyDamage_Event` :!signature `self.OnTakeAnyDamage`
  (params (DamagedActor :type "Actor Object Reference") (Damage :type "Float (single-precision)") (DamageType :type "DamageType Object Reference") (InstigatedBy :type "Controller Object Reference") (DamageCauser :type "Actor Object Reference"))
  (bind _returnvalue (* (`SceneComponent.GetForwardVector` (`Actor.RootComponent` (`self.PlayerRef`))) -1.0))
  (bind (_returnvalue_x _returnvalue_y _returnvalue_z) (`KismetMathLibrary.BreakVector` (* (`SceneComponent.GetForwardVector` (`Actor.RootComponent` (`self.PlayerRef`))) 30000.0)))
  (bind (_returnvalue_x_2 _returnvalue_y_2 _returnvalue_z_2) (`KismetMathLibrary.BreakVector` (* _returnvalue 20000.0)))
  (`/Engine/EditorBlueprintResources/StandardMacros.DoOnce` false :!label _label
    (:`Completed`
      (`AISense_Damage.ReportDamageEvent` DamagedActor InstigatedBy Damage (`self.K2_GetActorLocation`))
      (set `self.Health` (- (`self.Health`) Damage))
      (if (<= (`self.Health`) 0.0)
        (set `self.isDead` true)
        (`/Engine/EditorBlueprintResources/StandardMacros.DoOnce` false
          (:`Completed`
            (`BlackboardComponent.SetValueAsBool` (`AIController.Blackboard` (`AIBlueprintHelperLibrary.GetAIController` self)) (`self.isDead_BB_BoolName`) true)
            (`PrimitiveComponent.SetSimulatePhysics` (`self.Mesh`) true)
            (`PrimitiveComponent.SetCollisionResponseToChannel` (`self.CapsuleComponent`) "ECC_Pawn" "ECR_Ignore")
            (`PrimitiveComponent.SetCollisionResponseToChannel` (`self.CapsuleComponent`) "ECC_Camera" "ECR_Ignore")
            (`NiagaraFunctionLibrary.SpawnSystemAtLocation` "/Game/Pterafier/Niagara/NS_HitEffect.NS_HitEffect" (`self.K2_GetActorLocation`))
            (`GameplayStatics.PlaySoundAtLocation` "/Game/Pterafier/Sounds/547041__cogfirestudios__hit-swing-sword-small-3.547041__cogfirestudios__hit-swing-sword-small-3" (`self.K2_GetActorLocation`) (struct) (`KismetMathLibrary.RandomFloatInRange` 1.0 1.2) (`KismetMathLibrary.RandomFloatInRange` 0.95 1.1) 0.0 null null null null)
            (if (and (== _returnvalue_x 0.0) (== _returnvalue_y 0.0))
              (`PrimitiveComponent.AddImpulse` (`self.Mesh`) (+ _returnvalue (`KismetMathLibrary.MakeVector` _returnvalue_x_2 _returnvalue_y_2 (/ _returnvalue_z_2 2.0))) "None" false)
              (else
                (`PrimitiveComponent.AddImpulse` (`self.Mesh`) (`KismetMathLibrary.MakeVector` _returnvalue_x _returnvalue_y (/ _returnvalue_z 2.0)) "None" false)))
            (`KismetSystemLibrary.Delay` 5.0)
            (`self.K2_DestroyActor`)))
        (else
          (`|PlayMontage` (`self.Mesh`) "/Game/Animals_Warrior_Pack/Animations/1With_Weapon/Anim_Warrior_Get_Hit_2_Montage.Anim_Warrior_Get_Hit_2_Montage" 2.0
            (:`then`
              (`CharacterMovementComponent.SetMovementMode` (`self.CharacterMovement`) "MOVE_None" 0)
              (`NiagaraFunctionLibrary.SpawnSystemAtLocation` "/Game/Pterafier/Niagara/NS_HitEffect.NS_HitEffect" (`self.K2_GetActorLocation`))
              (`GameplayStatics.PlaySoundAtLocation` "/Game/Pterafier/Sounds/547041__cogfirestudios__hit-swing-sword-small-3.547041__cogfirestudios__hit-swing-sword-small-3" (`self.K2_GetActorLocation`) (struct) (`KismetMathLibrary.RandomFloatInRange` 1.0 1.2) (`KismetMathLibrary.RandomFloatInRange` 0.95 1.1) 0.0 null null null null)
              (`KismetSystemLibrary.Delay` 0.1)
              (goto _label :!via `Reset`))
            (:`OnCompleted`
              _)
            (:`OnInterrupted`
              _))
          (`CharacterMovementComponent.SetMovementMode` (`self.CharacterMovement`) "MOVE_Walking" 0))))))

(event `Attack`
  (bind _hitdetector (`self.HitDetector`))
  (`AIController.K2_SetFocus` (`AIBlueprintHelperLibrary.GetAIController` self) (`GameplayStatics.GetPlayerCharacter` 0))
  (`|PlayMontage` (`self.Mesh`) "/Game/Animals_Warrior_Pack/Animations/1With_Weapon/Anim_Warrior_Attack_4_Montage.Anim_Warrior_Attack_4_Montage" 5.0
    (:`OnNotifyBegin`
      (if (> (`self.Health`) 0.0)
        (bind _output_get (set `self.TraceEnd` (+ (`self.K2_GetActorLocation`) (* (`self.GetActorForwardVector`) 65.0))))
        (`KismetSystemLibrary.DrawDebugSphere` _output_get (`self.SphereTraceRadius`) 12 (struct :`G` 0.201321 :`B` 1.0 :`A` 1.0) 1.0)
        (`SceneComponent.K2_SetWorldLocation` _hitdetector (`self.TraceEnd`) false true)
        (for _array_element (`PrimitiveComponent.GetOverlappingActors` _hitdetector "/Game/ThirdPersonTemplate/ThirdPerson/Blueprints/BP_ThirdPersonCharacter.BP_ThirdPersonCharacter_C")
          (if (== _array_element (`self.PlayerRef`))
            (`GameplayStatics.ApplyDamage` (`self.PlayerStateRef`) (`self.Base Damage`) null self)))))))

(fn `GetPatrolRoute`
  (returns (PatrolRoute :type "/Game/Pterafier/Enemy/AI/BP_PatrolRoute Object Reference") (`UsePatrolRoute?` :type Boolean))
  (return (`self.PatrolRoute`) (`self.UsePatrolRoute?`)))

(fn `SetMovementSpeed`
  (params (Speed :type "/Game/Pterafier/Enemy/Enum/E_EnemyMovementState Enum" :default "NewEnumerator0"))
  (returns (SpeedValue :type "Float (double-precision)"))
  (bind _output_get (set `CharacterMovementComponent.MaxWalkSpeed` (select `/Game/Pterafier/Enemy/Enum/E_EnemyMovementState` Speed :`NewEnumerator1` 100.0 :`NewEnumerator2` 250.0 :!type "Float (single-precision)") (`self.CharacterMovement`)))
  (return _output_get))

(fn `UserConstructionScript`)